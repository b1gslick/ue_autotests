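; Test child of an inventory item Blueprint whose data and color are supplied from outside.
; SetInventoryData stores the passed inventory data and test color, then calls Init.
; GenerateColor returns the stored test color, and the construction script only calls its parent.
; BeginPlay and overlap events are disabled placeholders.
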(event Custom|SetInventoryData
  (params (InvData :type Inventory%20Data%20Structure) (Color :type Linear%20Color%20Structure))
  (Variables|Default|SetInventoryData InvData)
  (Variables|Default|SetTestColor Color)
  (CallFunction|Init))

(event EventBeginPlay
  (|CallParentFunction) ; This node is disabled and will not be called.\nDrag off pins to build functionality.
)

(event Collision|EventActorBeginOverlap
  (params (OtherActor :type Actor%20Object%20Reference))
  (|CallParentFunction OtherActor) ; This node is disabled and will not be called.\nDrag off pins to build functionality.
)

(fn ConstructionScript
  (|CallParentFunction))

(fn GenerateColor
  (return (Variables|Default|GetTestColor)))